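; Player character Blueprint that provides basic movement, mouse look and jumping.
; Forward and lateral axis inputs feed movement along directions derived from the control rotation's yaw only, so camera pitch does not affect movement.
; Turn and look-up axes drive controller yaw and pitch, and the jump action calls Jump on press.
; Overlap, Tick and the construction script are empty.
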(event Collision|EventActorBeginOverlap
  (params (OtherActor :type Actor%20Object%20Reference)))

(event EventTick
  (params (DeltaSeconds :type Float%20%28single-precision%29)))

(event Input|ActionEvents|InputActionSauter
  (params (Key :type Key%20Structure))
  ;[1 1 1] Saut
  (:Pressed
    (Character|Jump)))

(event Input|AxisEvents|InputAxisAvancer
  (params (AxisValue :type Float%20%28single-precision%29))
  ;[1 1 1] Mouvement
  (Pawn|Input|AddMovementInput (Math|Vector|GetForwardVector (Math|Rotator|MakeRotator 0.0 0.0 (.Yaw (Math|Rotator|BreakRotator (Pawn|GetControlRotation :!class /Script/Engine.Pawn))))) AxisValue false))

(event Input|AxisEvents|InputAxisDeplacementLateral
  (params (AxisValue :type Float%20%28single-precision%29))
  ;[1 1 1] Mouvement
  (Pawn|Input|AddMovementInput (Math|Vector|GetRightVector (Math|Rotator|MakeRotator 0.0 0.0 (.Yaw (Math|Rotator|BreakRotator (Pawn|GetControlRotation :!class /Script/Engine.Pawn))))) AxisValue false))

(event Input|AxisEvents|InputAxisturn
  (params (AxisValue :type Float%20%28single-precision%29))
  ;[1 1 1] Souris
  (Pawn|Input|AddControllerYawInput AxisValue))

(event Input|AxisEvents|InputAxisLookUp
  (params (AxisValue :type Float%20%28single-precision%29))
  ;[1 1 1] Souris
  (Pawn|Input|AddControllerPitchInput AxisValue))

(fn ConstructionScript)